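; Player character with axis-driven look and movement and a hold-E edit mode for nearby special actors and material planes.
; While E is held, Tick checks capsule overlaps, storing and showing each BP_SpecialActor.
; Overlapped BP_MaterialPlanes get custom depth and call Change, after custom depth is cleared on the stored actor's linked static mesh.
; Camera trace and hide/reset logic are disconnected and never run.
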(event `self.ReceiveTick`
  (params (DeltaSeconds :type "Float (single-precision)"))
  (if (`self.Editable`)
    (`|ExecutionSequence`
      (:`then_0`
        (for _array_element (`PrimitiveComponent.GetOverlappingActors` (`self.Capsule`) "/Game/Importado/Blueprints/BP_SpecialActor.BP_SpecialActor_C")
          (bind _asbp_special_actor (cast `/Game/Importado/Blueprints/BP_SpecialActor` _array_element))
          (bind _output_get (set `self.Actor` _asbp_special_actor))
          (`/Game/Importado/Blueprints/BP_SpecialActor.Show` _output_get)))
      (:`then_1`
        (for _array_element_2 (`PrimitiveComponent.GetOverlappingActors` (`self.Capsule`) "/Game/Importado/Blueprints/BP_MaterialPlane.BP_MaterialPlane_C")
          (bind _asbp_material_plane (cast `/Game/Importado/Blueprints/BP_MaterialPlane` _array_element_2))
          (`PrimitiveComponent.SetRenderCustomDepth` (`/Game/Importado/Blueprints/BP_MaterialPlane.StaticMesh` _asbp_material_plane) true)
          (bind _asstatic_mesh_actor (cast `StaticMeshActor` (`/Game/Importado/Blueprints/BP_SpecialActor.Actor` (`self.Actor`))))
          (`PrimitiveComponent.SetRenderCustomDepth` (`StaticMeshActor.StaticMeshComponent` _asstatic_mesh_actor) false)
          (`/Game/Importado/Blueprints/BP_MaterialPlane.Change` _asbp_material_plane))))))

(event `Key|E`
  (params (Key :type "Key Structure" :default "AnyKey"))
  (:`Pressed`
    (set `self.Editable` true))
  (:`Released`
    (set `self.Editable` false)))

(event `InputAxis|XAxis`
  (params (AxisValue :type "Float (single-precision)"))
  (`self.AddControllerYawInput` (* AxisValue 0.5)))

(event `InputAxis|YAxis`
  (params (AxisValue :type "Float (single-precision)"))
  (`self.AddControllerPitchInput` (* AxisValue -0.5)))

(event `InputAxis|Forward`
  (params (AxisValue :type "Float (single-precision)"))
  (`self.AddMovementInput` (`KismetMathLibrary.GetForwardVector` (`self.GetControlRotation`)) (* AxisValue 0.5)))

(event `InputAxis|Sides`
  (params (AxisValue :type "Float (single-precision)"))
  (`self.AddMovementInput` (`KismetMathLibrary.GetRightVector` (`self.GetControlRotation`)) (* AxisValue 0.5)))

(fn `UserConstructionScript`)