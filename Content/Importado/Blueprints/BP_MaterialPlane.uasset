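; BP_MaterialPlane is an actor that displays one material on two static meshes and asks a referenced object to change to it.
; SetMaterial applies the material to both meshes and stores the reference and index.
; Change alternates through a looping MultiGate: one call runs ChangeMaterial with that index behind a DoOnce.
; The next waits on a short retriggerable delay, disables the first mesh's custom depth and resets the DoOnce.
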(event `SetMaterial`
  (params (Material :type "MaterialInterface Object Reference") (Reference :type "/Game/Importado/Blueprints/BP_SpecialActor Object Reference") (Index :type Integer))
  (set `self.Index` Index)
  (set `self.Reference` Reference)
  (`PrimitiveComponent.SetMaterial` (`self.StaticMesh`) 0 Material)
  (`PrimitiveComponent.SetMaterial` (`self.StaticMesh1`) 0 Material))

(event `Change`
  (`|MultiGate` false true
    (:`Out 0`
      (`/Engine/EditorBlueprintResources/StandardMacros.DoOnce` false :!label _label
        (:`Completed`
          (`KismetSystemLibrary.PrintString` "PRECHANGE")
          (`/Game/Importado/Blueprints/BP_SpecialActor.ChangeMaterial` (`self.Reference`) (`self.Index`)))))
    (:`Out 1`
      (`KismetSystemLibrary.RetriggerableDelay` 0.2)
      (`PrimitiveComponent.SetRenderCustomDepth` (`self.StaticMesh`) false)
      (goto _label :!via `Reset`))))

(fn `UserConstructionScript`)