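; BP_SpecialActor is a material picker for a referenced StaticMeshActor, with thumbnail tiles that face the player's camera.
; Show alternates via MultiGate between enabling custom-depth stencil with a row of BP_MaterialPlane tiles, spawned alternately either side of center, and calling Hide after a short delay.
; Each tile receives its index and a self reference.
; ChangeMaterial applies that index's group of NumMaterials entries from Materials to the mesh's slots.
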(event `ChangeMaterial`
  (params (Index :type Integer))
  (bind _nummaterials (`self.NumMaterials`))
  (`KismetSystemLibrary.PrintString` (`KismetStringLibrary.Conv_IntToString` Index))
  (for (_array_element _array_index) (`self.Materials`)
    (if (== Index (/ _array_index _nummaterials))
      (bind _asstatic_mesh_actor (cast `StaticMeshActor` (`self.Actor`)))
      (`PrimitiveComponent.SetMaterial` (`StaticMeshActor.StaticMeshComponent` _asstatic_mesh_actor) (mod _array_index _nummaterials) _array_element))))

(event `self.ReceiveTick`
  (params (DeltaSeconds :type "Float (single-precision)"))
  (bind _asbp_character (cast `/Game/Importado/Blueprints/BP_Character` (`Controller.K2_GetPawn` (`GameplayStatics.GetPlayerController` 0))))
  (`SceneComponent.K2_SetWorldRotation` (`self.ForTiles`) (`KismetMathLibrary.FindLookAtRotation` (`SceneComponent.K2_GetComponentLocation` (`self.ForTiles`)) (`SceneComponent.K2_GetComponentLocation` (`/Game/Importado/Blueprints/BP_Character.Camera` _asbp_character))) false false))

(event `Show`
  (`|MultiGate` false true
    (:`Out 0`
      (`/Engine/EditorBlueprintResources/StandardMacros.DoOnce` false :!label _label
        (:`Completed`
          (`KismetSystemLibrary.PrintString` "OUT1")
          (bind _asstatic_mesh_actor (cast `StaticMeshActor` (`self.Actor`)))
          (bind _staticmeshcomponent (`StaticMeshActor.StaticMeshComponent` _asstatic_mesh_actor))
          (`PrimitiveComponent.SetRenderCustomDepth` _staticmeshcomponent true)
          (`PrimitiveComponent.SetCustomDepthStencilValue` _staticmeshcomponent 252)
          (for (_array_element _array_index) (`self.MaterialsForThumb`)
            (bind _returnvalue (`|SpawnActorFromClass` "/Game/Importado/Blueprints/BP_MaterialPlane.BP_MaterialPlane_C" (`KismetMathLibrary.MakeTransform` (`KismetMathLibrary.MakeVector` 0.0 (* (* (+ (* (/ _array_index 2) 2) 1) (select `int` (mod _array_index 2) :`0` 1.0 :`1` -1.0)) 17.0)) (struct) (0.3 0.3 0.3)) "Undefined" "OverrideRootScale" self))
            (`/Game/Importado/Blueprints/BP_MaterialPlane.SetMaterial` _returnvalue _array_element self _array_index)
            (`SceneComponent.K2_AttachTo` (`/Game/Importado/Blueprints/BP_MaterialPlane.Box` _returnvalue) (`self.ForTiles`) "None" "KeepRelativeOffset" true)
            (`KismetArrayLibrary.Array_Add` (`self.Tiles`) _returnvalue)))))
    (:`Out 1`
      (`KismetSystemLibrary.RetriggerableDelay` 0.2)
      (`KismetSystemLibrary.PrintString` "OUT2")
      (`self.Hide`)
      (goto _label :!via `Reset`))))

(event `Hide`
  (bind _asstatic_mesh_actor (cast `StaticMeshActor` (`self.Actor`)))
  (`PrimitiveComponent.SetRenderCustomDepth` (`StaticMeshActor.StaticMeshComponent` _asstatic_mesh_actor) false)
  (for _array_element (`self.Tiles`)
    (`self.K2_DestroyActor` _array_element)))

(fn `UserConstructionScript`
  (`BoxComponent.SetBoxExtent` (`self.Box`) (`self.BoxSize`) true)
  (`SceneComponent.K2_SetRelativeLocation` (`self.ForTiles`) (`self.RelativeLocation`) false false))